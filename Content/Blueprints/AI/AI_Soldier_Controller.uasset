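; AI controller for soldier enemies that runs the soldier behavior tree and feeds perception results into its blackboard.
; On each perception update, UpdateSenses maps every updated actor's last stimuli by array index, relying on sense order.
; The first sets player visibility, the second sound investigation and target location.
; A successful third flags being shot and targets the player's current position, whatever the source.
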(event `self.ReceiveBeginPlay`
  (`self.RunBehaviorTree` "/Game/Blueprints/AI/AI_Solider_BT.AI_Solider_BT"))

(event `self.AIPerception.OnTargetPerceptionUpdated`
  (params (Actor :type "Actor Object Reference") (Stimulus :type "AIStimulus Structure")))

(event `self.AIPerception.OnPerceptionUpdated`
  (params (UpdatedActors :type "Array of Actor Object Reference (by ref)"))
  (for _array_element UpdatedActors
    (bind _info (`AIPerceptionComponent.GetActorsPerception` (`self.AIPerception`) _array_element))
    (`self.UpdateSenses` (`.LastSensedStimuli` (break `ActorPerceptionBlueprintInfo` _info)))))

(fn `UpdateSenses`
  (params (Array :type "Array of AIStimulus Structure"))
  (locals (sense :type "AIStimulus Structure"))
  (bind _returnvalue (`AIBlueprintHelperLibrary.GetBlackboard` null))
  (bind _returnvalue_2 (`AIBlueprintHelperLibrary.GetBlackboard` null))
  (bind (_sense_age _sense_expirationage _sense_strength _sense_stimuluslocation _sense_receiverlocation _sense_tag _sense_bsuccessfullysensed) (break `AIStimulus` (`local.sense`)))
  (for (_array_element _array_index) Array
    (set `local.sense` _array_element)
    (switch `int` _array_index
      (:`0`
        (`BlackboardComponent.SetValueAsBool` (`AIBlueprintHelperLibrary.GetBlackboard` null) "PlayerInView?" _sense_bsuccessfullysensed))
      (:`1`
        (`BlackboardComponent.SetValueAsVector` _returnvalue_2 "TargetLocation" _sense_stimuluslocation)
        (`BlackboardComponent.SetValueAsBool` _returnvalue_2 "InvestigatingSound?" _sense_bsuccessfullysensed)
        (`KismetSystemLibrary.PrintString` (`KismetStringLibrary.Conv_BoolToString` _sense_bsuccessfullysensed)))
      (:`2`
        (if _sense_bsuccessfullysensed
          (`BlackboardComponent.SetValueAsBool` _returnvalue "Shot?" true)
          (`BlackboardComponent.SetValueAsVector` _returnvalue "TargetLocation" (`self.K2_GetActorLocation` (`GameplayStatics.GetPlayerCharacter` 0)))
          (`BlackboardComponent.SetValueAsBool` _returnvalue "InvestigatingSound?" true))))))

(fn `UserConstructionScript`)