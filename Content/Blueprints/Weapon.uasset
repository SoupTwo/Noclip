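; Weapon is an actor with a static mesh that plays a drop sound on hard impacts and destroys itself ten seconds after BeginPlay.
; Component hits above a normal impulse threshold play the attenuated cue at the impact point, with volume mapped from impulse strength.
; A DoOnce that resets after a short delay throttles repeated impact sounds.
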(event `self.ReceiveBeginPlay`
  (`KismetSystemLibrary.Delay` 10.0)
  (`self.K2_DestroyActor`))

(event `self.StaticMesh.OnComponentHit`
  (params (HitComponent :type "PrimitiveComponent Object Reference") (OtherActor :type "Actor Object Reference") (OtherComp :type "PrimitiveComponent Object Reference") (NormalImpulse :type "Vector Structure") (Hit :type "HitResult Structure (by ref)"))
  (bind _returnvalue (`KismetMathLibrary.VSize` NormalImpulse))
  (if (> _returnvalue 180.0)
    (`/Engine/EditorBlueprintResources/StandardMacros.DoOnce` false :!label _label
      (:`Completed`
        (`GameplayStatics.PlaySoundAtLocation` "/Game/Sound/Weapon_Drop_Cue.Weapon_Drop_Cue" (`.Location` (`GameplayStatics.BreakHitResult` Hit)) (struct) (`KismetMathLibrary.MapRangeClamped` _returnvalue 180.0 210.0 0.9 1.15) 1.0 0.0 "/Game/Sound/Weapon_Drop_Attenuation.Weapon_Drop_Attenuation" null null)
        (`KismetSystemLibrary.Delay` 0.05)
        (goto _label :!via `Reset`)))))

(fn `UserConstructionScript`)