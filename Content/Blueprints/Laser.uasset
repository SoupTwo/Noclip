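; Laser Blueprint that keeps a laser effect pointed at the first player character.
; Each Tick it rotates the Laser component toward the character and runs a Visibility line trace to their location, with debug drawing on.
; The trace's hit distance feeds the effect's "Distance" float variable.
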(event `self.ReceiveTick`
  (params (DeltaSeconds :type "Float (single-precision)"))
  (bind _returnvalue (`GameplayStatics.GetPlayerCharacter` 0))
  (`/Engine/EditorBlueprintResources/StandardMacros.IsValid` _returnvalue
    (:`Is Valid`
      (`SceneComponent.K2_SetWorldRotation` (`self.Laser`) (`KismetMathLibrary.Conv_VectorToRotator` (`KismetMathLibrary.GetDirectionUnitVector` (`SceneComponent.K2_GetComponentLocation` (`self.Laser`)) (`self.K2_GetActorLocation` (`GameplayStatics.GetPlayerCharacter` 0)))) false false)
      (bind _outhit (`KismetSystemLibrary.LineTraceSingle` :`Start` (`SceneComponent.K2_GetComponentLocation` (`self.Laser`)) :`End` (`self.K2_GetActorLocation` _returnvalue) :`TraceChannel` "TraceTypeQuery1" :`DrawDebugType` "ForOneFrame" :`DrawTime` 0.0))
      (`NiagaraComponent.SetVariableFloat` (`self.Laser`) "Distance" (`.Distance` (`GameplayStatics.BreakHitResult` _outhit))))))

(fn `UserConstructionScript`)